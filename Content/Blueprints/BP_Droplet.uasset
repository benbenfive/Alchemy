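; BP_Droplet is a small liquid droplet carrying color, capacity and effects, set by Construct along with a tinted water material.
; On overlap, it ignores its Dropper and absorbs other droplets, summing capacity and blending color by capacity weights.
; A Got flag stops absorbed droplets from processing further overlaps.
; It pours into cauldrons (amount, color) or bottles (also material, effects), then destroys itself, as it does on anything else except VR_Pawn.
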(event EventBeginPlay)

(event Collision|EventActorBeginOverlap
  (params (OtherActor :type Actor%20Object%20Reference))
  (bind _returnvalue (Utilities|GetClass OtherActor))
  (if (not (== (Variables|Default|Getdropper) OtherActor))
    (if (not (Variables|Default|Getgot))
      (if (Utilities|ClassIsChildOf _returnvalue "BP_Droplet_C")
        (bind _asbp_droplet (Utilities|Casting|CastToBP_Droplet OtherActor))
        (bind (_capacity _color) (CallFunction|Get _asbp_droplet))
        (Variables|Default|Setcapacity (+ _capacity (Variables|Default|Getcapacity)))
        (Variables|Default|Setcolor (+ (* _color (/ _capacity (+ _capacity (Variables|Default|Getcapacity)))) (* (Variables|Default|Getcolor) (/ (Variables|Default|Getcapacity) (+ _capacity (Variables|Default|Getcapacity))))))
        (Actor|DestroyActor OtherActor)
        (elif (Utilities|ClassIsChildOf _returnvalue "/Game/Blueprints/BP_Cauldron.BP_Cauldron_C")
          (bind _asbp_cauldron (Utilities|Casting|CastToBP_Cauldron OtherActor))
          (Default|ChangeWaterLevel _asbp_cauldron (Variables|Default|Getcapacity) (Variables|Default|Getcolor))
          (Actor|DestroyActor :!label _label)
          (elif (Utilities|ClassIsChildOf _returnvalue "/Game/Blueprints/BP_Bottle_Base.BP_Bottle_Base_C")
            (bind _asbp_bottle_base (Utilities|Casting|CastToBP_Bottle_Base OtherActor))
            (Default|AddLiquid _asbp_bottle_base (Rendering|Material|GetMaterial (Variables|Default|GetCube) 0) (Variables|Default|Geteffects) (Variables|Default|Getcapacity) (Variables|Default|Getcolor))
            (goto _label)
            (elif (not (Utilities|ClassIsChildOf _returnvalue "/Game/Blueprints/VR_Pawn.VR_Pawn_C"))
              (goto _label))))))))

(event EventTick
  (params (DeltaSeconds :type Float%20%28single-precision%29)))

(fn ConstructionScript
  (Transformation|SetWorldScale3D (Variables|Default|GetCube) "0.025000,0.025000,0.025000"))

(fn Construct
  (params (color :type Linear%20Color%20Structure) (capacity :type Float%20%28single-precision%29) (effects :type String) (dropper :type Actor%20Object%20Reference))
  (Variables|Default|Setcolor color)
  (Variables|Default|Setcapacity capacity)
  (Variables|Default|Seteffects effects)
  (Variables|Default|Setdropper dropper)
  (bind _returnvalue (Rendering|Material|CreateDynamicMaterialInstance (Variables|Default|GetCube) 0 "/Game/Materials/M_Water_Lake.M_Water_Lake" "None" :!class /Script/Engine.PrimitiveComponent))
  (Rendering|Material|SetVectorParameterValue _returnvalue "Color" color :!class /Script/Engine.MaterialInstanceDynamic)
  (Rendering|Material|SetMaterial (Variables|Default|GetCube) 0 _returnvalue)
  (Rendering|SetVisibility (Variables|Default|GetCube) true true))

(fn Get
  (Variables|Default|Setgot true)
  (return (Variables|Default|Getcapacity) (Variables|Default|Getcolor) (Variables|Default|Geteffects)))