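; BP_Cauldron is a cauldron actor that absorbs dropped ingredients and tints its water with their colors.
; On overlap, a BP_Ingredient whose mesh is simulating physics is blended into the stored Color at one-third weight, then destroyed.
; Each blend creates a dynamic material instance on DurpCauldronWater to apply the result through the Color parameter.
; The construction script sets the starting water color.
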(event EventBeginPlay)

(event Collision|EventActorBeginOverlap
  (params (OtherActor :type Actor%20Object%20Reference))
  (if (Utilities|ClassIsChildOf (Utilities|GetClass OtherActor) "/Game/Blueprints/BP_Ingredient.BP_Ingredient_C")
    (bind _asbp_ingredient (Utilities|Casting|CastToBP_Ingredient OtherActor))
    (if (Physics|IsSimulatingPhysics (Variables|/Game/Blueprints/BP_Pickupable.BP_Pickupable_C|GetMesh _asbp_ingredient) "None")
      (bind _returnvalue (Rendering|Material|CreateDynamicMaterialInstance (Variables|Default|Getdurp_cauldron_water) 0 (Rendering|Material|GetMaterial (Variables|Default|Getdurp_cauldron_water) 0) "None" :!class /Script/Engine.PrimitiveComponent))
      (bind _color (Default|GetColor _asbp_ingredient))
      (bind _output_get (Variables|Default|Setcolor (+ (/ _color "(R=3.000000,G=3.000000,B=3.000000,A=3.000000)") (+ (/ (Variables|Default|Getcolor) "(R=3.000000,G=3.000000,B=3.000000,A=3.000000)") (/ (Variables|Default|Getcolor) "(R=3.000000,G=3.000000,B=3.000000,A=3.000000)")))))
      (Rendering|Material|SetVectorParameterValue _returnvalue "Color" _output_get :!class /Script/Engine.MaterialInstanceDynamic)
      (Rendering|Material|SetMaterialbyName (Variables|Default|Getdurp_cauldron_water) "None" _returnvalue)
      (Actor|DestroyActor _asbp_ingredient))))

(event EventTick
  (params (DeltaSeconds :type Float%20%28single-precision%29)))

(fn ConstructionScript
  (Variables|Default|Setcolor "(R=0.301961,G=0.352941,B=0.439216,A=1.000000)"))