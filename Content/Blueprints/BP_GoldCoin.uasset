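; BP_GoldCoin is a gold coin Blueprint that responds to an Interact event.
; When Interact fires with Holding true, it destroys the coin's Mesh component, leaving the actor itself in place.
; BeginPlay, overlap and Tick are disabled stubs, and the construction script only calls its parent.
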(event EventBeginPlay
  (|CallParentFunction) ; This node is disabled and will not be called.\nDrag off pins to build functionality.
)

(event Collision|EventActorBeginOverlap
  (params (OtherActor :type Actor%20Object%20Reference))
  (|CallParentFunction OtherActor) ; This node is disabled and will not be called.\nDrag off pins to build functionality.
)

(event EventTick
  (params (DeltaSeconds :type Float%20%28single-precision%29))
  (|CallParentFunction DeltaSeconds) ; This node is disabled and will not be called.\nDrag off pins to build functionality.
)

(event EventInteract
  (params (hand :type Scene%20Component%20Object%20Reference) (bHolding :type Boolean))
  (if bHolding
    (Components|DestroyComponent (Variables|Character|GetMesh))))

(fn ConstructionScript
  (|CallParentFunction))