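; VR pawn that grabs pickupables and gathers handfuls of coins with either motion controller.
; Grab takes all coins in the hand's box if the first overlap is a coin, otherwise messages that item; trigger adds one while holding coins.
; Each hand keeps a count with a randomized limit that spills coins when reached; only the right still picks up afterwards.
; Release spawns a gold coin per count, thrown at controller velocity.
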(event EventBeginPlay)

(event Collision|EventActorBeginOverlap
  (params (OtherActor :type Actor%20Object%20Reference)))

(event EventTick
  (params (DeltaSeconds :type Float%20%28single-precision%29)))

(event Input|ActionEvents|InputActionGrabLeft
  (params (Key :type Key%20Structure :default "None"))
  (bind _boxleft (Variables|Default|GetBoxLeft))
  (bind _overlappingactors (Collision|GetOverlappingActors _boxleft "/Game/Blueprints/BP_Pickupable.BP_Pickupable_C" :!class /Script/Engine.PrimitiveComponent))
  (bind _output (Utilities|Array|Get(acopy) _overlappingactors))
  (:Pressed
    (Variables|Default|SetbHolding_L true)
    (if (Utilities|ClassIsChildOf (Utilities|GetClass _output) "/Game/Blueprints/BP_BaseCoin.BP_BaseCoin_C")
      (for _array_element (Collision|GetOverlappingActors (Variables|Default|GetBoxLeft) "/Game/Blueprints/BP_BaseCoin.BP_BaseCoin_C" :!class /Script/Engine.PrimitiveComponent)
        (CallFunction|PickupCoin _array_element true))
      (else
        (Class|Interactable|Interact(Message) _output (Variables|Default|GetMotionController_left) (Variables|Default|GetbHolding_L) :!label _label))))
  (:Released
    (Variables|Default|SetbHolding_L false)
    (if (> (Variables|Default|GetnumCoins_L) 0)
      (for _index (range 1 (Variables|Default|GetnumCoins_L))
        (CallFunction|DropCoin true))
      (Variables|Default|SetnumCoins_L 0)
      (else
        (goto _label)))))

(event Input|ActionEvents|InputActionGrabRight
  (params (Key :type Key%20Structure :default "None"))
  (bind _boxright (Variables|Default|GetBoxRight))
  (bind _overlappingactors (Collision|GetOverlappingActors _boxright "/Game/Blueprints/BP_Pickupable.BP_Pickupable_C" :!class /Script/Engine.PrimitiveComponent))
  (bind _output (Utilities|Array|Get(acopy) _overlappingactors))
  (:Pressed
    (Variables|Default|SetbHolding_R true)
    (if (Utilities|ClassIsChildOf (Utilities|GetClass _output) "/Game/Blueprints/BP_BaseCoin.BP_BaseCoin_C")
      (for _array_element (Collision|GetOverlappingActors (Variables|Default|GetBoxRight) "/Game/Blueprints/BP_BaseCoin.BP_BaseCoin_C" :!class /Script/Engine.PrimitiveComponent)
        (CallFunction|PickupCoin _array_element false))
      (else
        (Class|Interactable|Interact(Message) _output (Variables|Default|GetMotionController_right) (Variables|Default|GetbHolding_R) :!label _label))))
  (:Released
    (Variables|Default|SetbHolding_R false)
    (if (> (Variables|Default|GetnumCoins_R) 0)
      (for _index (range 1 (Variables|Default|GetnumCoins_R))
        (CallFunction|DropCoin false))
      (Variables|Default|SetnumCoins_R 0)
      (else
        (goto _label)))))

(event Input|ActionEvents|InputActionTriggerLeft
  (params (Key :type Key%20Structure :default "None"))
  (:Pressed
    (if (> (Variables|Default|GetnumCoins_L) 0)
      (bind _array_element (Utilities|Array|ForEachLoopwithBreak (Collision|GetOverlappingActors (Variables|Default|GetBoxLeft) "/Game/Blueprints/BP_BaseCoin.BP_BaseCoin_C" :!class /Script/Engine.PrimitiveComponent) :!label _label)
        (:LoopBody
          (if (Utilities|ClassIsChildOf (Utilities|GetClass _array_element) "/Game/Blueprints/BP_BaseCoin.BP_BaseCoin_C")
            (CallFunction|PickupCoin _array_element true)
            (goto _label Break)))))))

(event Input|ActionEvents|InputActionTriggerRight
  (params (Key :type Key%20Structure :default "None"))
  (:Pressed
    (if (> (Variables|Default|GetnumCoins_R) 0)
      (bind _array_element (Utilities|Array|ForEachLoopwithBreak (Collision|GetOverlappingActors (Variables|Default|GetBoxRight) "/Game/Blueprints/BP_BaseCoin.BP_BaseCoin_C" :!class /Script/Engine.PrimitiveComponent) :!label _label)
        (:LoopBody
          (if (Utilities|ClassIsChildOf (Utilities|GetClass _array_element) "/Game/Blueprints/BP_BaseCoin.BP_BaseCoin_C")
            (CallFunction|PickupCoin _array_element false)
            (goto _label Break)))))))

(fn ConstructionScript)

(fn PickupCoin
  (params (coin :type Object%20Object%20Reference) (leftHand :type Boolean))
  (bind _returnvalue (Math|Random|RandomIntegerinRange 1 5))
  (bind _numcoins_r (Variables|Default|GetnumCoins_R))
  (bind _numcoins_l (Variables|Default|GetnumCoins_L))
  (bind _returnvalue_2 (+ _returnvalue 20))
  (if leftHand
    (if (< _numcoins_l _returnvalue_2)
      (Math|Integer|IncrementInt _numcoins_l
        (:%20%20
          (Class|Interactable|Interact(Message) coin (Variables|Default|GetMotionController_left) (Variables|Default|GetbHolding_L))))
      (else
        (for _index (range 1 (Math|Random|RandomIntegerinRange 1 3))
          (CallFunction|DropCoin true)
          (Math|Integer|DecrementInt _numcoins_l))))
    (else
      (if (< _numcoins_r _returnvalue_2)
        _
        (else
          (for _index_2 (range 1 (Math|Random|RandomIntegerinRange 1 3))
            (CallFunction|DropCoin false)
            (Math|Integer|DecrementInt _numcoins_r))))
      (Math|Integer|IncrementInt _numcoins_r
        (:%20%20
          (Class|Interactable|Interact(Message) coin (Variables|Default|GetMotionController_right) (Variables|Default|GetbHolding_R)))))))

(fn DropCoin
  (params (leftHand :type Boolean))
  (bind _motioncontroller_right (Variables|Default|GetMotionController_right))
  (bind _motioncontroller_left (Variables|Default|GetMotionController_left))
  (if leftHand
    (bind _returnvalue (Game|SpawnActorfromClass "/Game/Blueprints/BP_GoldCoin.BP_GoldCoin_C" (Math|Transform|MakeTransform (Transformation|GetWorldLocation _motioncontroller_left) (Transformation|GetWorldRotation _motioncontroller_left)) "AdjustIfPossibleButAlwaysSpawn" 0 0))
    (Class|PrimitiveComponent|SetAllPhysicsLinearVelocity (Variables|/Game/Blueprints/BP_Pickupable.BP_Pickupable_C|GetMesh _returnvalue) (Transformation|GetComponentVelocity _motioncontroller_left) false)
    (else
      (bind _returnvalue_2 (Game|SpawnActorfromClass "/Game/Blueprints/BP_GoldCoin.BP_GoldCoin_C" (Math|Transform|MakeTransform (Transformation|GetWorldLocation _motioncontroller_right) (Transformation|GetWorldRotation _motioncontroller_right)) "AdjustIfPossibleButAlwaysSpawn" 0 0))
      (Class|PrimitiveComponent|SetAllPhysicsLinearVelocity (Variables|/Game/Blueprints/BP_Pickupable.BP_Pickupable_C|GetMesh _returnvalue_2) (Transformation|GetComponentVelocity _motioncontroller_right) false))))