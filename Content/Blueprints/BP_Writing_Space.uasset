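; BP_Writing_Space is an actor that counts feathers entering its overlap area and shows the running count as text.
; On actor overlap it checks whether the other actor's class derives from BP_Feather, then increments Quantity and writes it to QuantityText.
; The construction script shrinks the Box component to a tenth of its scale in world space.
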(event EventBeginPlay)

(event Collision|EventActorBeginOverlap
  (params (OtherActor :type Actor%20Object%20Reference))
  (if (Utilities|ClassIsChildOf (Utilities|GetClass OtherActor) "/Game/Blueprints/BP_Feather.BP_Feather_C")
    (bind _result (Math|Integer|IncrementInt (Variables|Default|Getquantity))
      (:%20%20
        (Rendering|Components|TextRender|SetText (Variables|Default|GetQuantity_Text) (Utilities|Text|ToText(String) (Utilities|String|ToString(Integer) _result)))))))

(event EventTick
  (params (DeltaSeconds :type Float%20%28single-precision%29)))

(fn ConstructionScript
  (Transformation|SetWorldScale3D (Variables|Default|GetBox) "0.100000,0.100000,0.100000"))