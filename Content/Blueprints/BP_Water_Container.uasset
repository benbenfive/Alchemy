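; BP_Water_Container is a liquid container that tracks an amount against a capacity, along with the liquid's color and effects.
; AddLiquid applies a positive or negative change clamped between empty and full, then stores the incoming effects.
; The amount actually changed serves directly as the color blend weight, without normalization.
; Each visual update creates a new M_Water_Lake dynamic material for the Cube and sets its Color parameter.
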(event EventBeginPlay)

(event Collision|EventActorBeginOverlap
  (params (OtherActor :type Actor%20Object%20Reference)))

(event EventTick
  (params (DeltaSeconds :type Float%20%28single-precision%29)))

(fn ConstructionScript)

(fn AddLiquid
  (params (amount :type Float%20%28single-precision%29) (color :type Linear%20Color%20Structure) (effects :type String))
  (bind _percent_change (CallFunction|ChangeWaterLevel amount))
  (CallFunction|UpdateWaterVisuals _percent_change color)
  (Variables|Default|Seteffects effects))

(fn ChangeWaterLevel
  (params (amount_changed :type Float%20%28single-precision%29))
  (bind _capacity (Variables|Default|Getcapacity))
  (LocalVariables|Setold (Variables|Default|Getamount))
  (if (> amount_changed 0.0)
    (if (> _capacity (Variables|Default|Getamount))
      (if (< (+ amount_changed (Variables|Default|Getamount)) _capacity)
        (Variables|Default|Setamount (+ amount_changed (Variables|Default|Getamount)) :!label _label)
        (else
          (Variables|Default|Setamount _capacity)))
      (return (- (Variables|Default|Getamount) (LocalVariables|Getold))))
    (elif (> (Variables|Default|Getamount) 0.0)
      (if (>= (+ amount_changed (Variables|Default|Getamount)) 0.0)
        (goto _label)
        (else
          (Variables|Default|Setamount 0.0)
          (return (- (Variables|Default|Getamount) (LocalVariables|Getold))))))))

(fn UpdateWaterVisuals
  (params (percent :type Float%20%28single-precision%29) (color :type Linear%20Color%20Structure))
  (bind _returnvalue (Rendering|Material|CreateDynamicMaterialInstance (Variables|Default|GetCube) 0 "/Game/Materials/M_Water_Lake.M_Water_Lake" "None" :!class /Script/Engine.PrimitiveComponent))
  (bind _output_get (Variables|Default|Setcolor (+ (* color percent) (* (Variables|Default|Getcolor) (- 1.0 percent)))))
  (Rendering|Material|SetVectorParameterValue _returnvalue "Color" _output_get :!class /Script/Engine.MaterialInstanceDynamic)
  (Rendering|Material|SetMaterialbyName (Variables|Default|GetCube) "None" _returnvalue))