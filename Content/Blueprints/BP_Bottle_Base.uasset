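; Base bottle actor that holds an amount of colored liquid with effects and pours it out when tipped.
; On Tick, rolling past 45 degrees spawns a BP_Droplet; tilt-scaled volume exceeding the empty space is drained into it along with color and effects.
; Added liquid is clamped to capacity, replaces the effects, and updates the color through a dynamic material instance using a percentage-weighted blend.
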(event EventBeginPlay
  (|CallParentFunction) ; This node is disabled and will not be called.\nDrag off pins to build functionality.
)

(event Collision|EventActorBeginOverlap
  (params (OtherActor :type Actor%20Object%20Reference))
  (|CallParentFunction OtherActor) ; This node is disabled and will not be called.\nDrag off pins to build functionality.
)

(event EventTick
  (params (DeltaSeconds :type Float%20%28single-precision%29))
  (bind _self self)
  (bind _bottle (Variables|Default|GetBottle))
  (bind _color (Variables|Default|Getcolor))
  (bind _returnvalue (Transformation|GetWorldRotation _bottle))
  (if (and (> (Variables|Default|Getamount) 0.0) (or (> (.roll _returnvalue) 45.0) (< (.roll _returnvalue) -45.0)))
    (bind _returnvalue_2 (Game|SpawnActorfromClass "/Game/Blueprints/BP_Droplet.BP_Droplet_C" (Transformation|GetWorldTransform (Variables|Default|Getdroplet_spawnpoint)) "AlwaysSpawn" 0 0))
    (bind _percent (CallFunction|PercentTipped (.roll _returnvalue)))
    (if (> (Math|Conversions|ToFloat(Integer) (Math|Float|Truncate (* _percent (Variables|Default|Getcapacity)))) (- (Variables|Default|Getcapacity) (Variables|Default|Getamount)))
      (bind _output_get (Variables|Default|Setamount (- (Variables|Default|Getamount) (- (Math|Conversions|ToFloat(Integer) (Math|Float|Truncate (* _percent (Variables|Default|Getcapacity)))) (- (Variables|Default|Getcapacity) (Variables|Default|Getamount))))))
      (if (<= _output_get 0.0)
        (Default|Construct _returnvalue_2 _color (+ _output_get (- (Math|Conversions|ToFloat(Integer) (Math|Float|Truncate (* _percent (Variables|Default|Getcapacity)))) (- (Variables|Default|Getcapacity) (Variables|Default|Getamount)))) (Variables|Default|Geteffects) _self)
        (Variables|Default|Setamount 0.0)
        (Variables|Default|Seteffects "")
        (Rendering|Material|SetMaterial (Variables|Default|GetLiquid) 0 "/Engine/BasicShapes/BasicShapeMaterial.BasicShapeMaterial")
        (else
          (Default|Construct _returnvalue_2 _color (- (Math|Conversions|ToFloat(Integer) (Math|Float|Truncate (* _percent (Variables|Default|Getcapacity)))) (- (Variables|Default|Getcapacity) (Variables|Default|Getamount))) (Variables|Default|Geteffects) _self)))
      (|CallParentFunction DeltaSeconds))))

(fn ConstructionScript
  (|CallParentFunction))

(fn AddLiquid
  (params (material :type Material%20Interface%20Object%20Reference) (effects :type String) (amount :type Float%20%28single-precision%29) (color :type Linear%20Color%20Structure))
  (if (== (Variables|Default|Getamount) 0.0)
    (Rendering|Material|SetMaterial (Variables|Default|GetLiquid) 0 material))
  (CallFunction|ChangeWaterLevel amount color)
  (Variables|Default|Seteffects effects))

(fn GetCapacity
  (return (Variables|Default|Getcapacity)))

(fn PercentTipped
  (params (x :type Float%20%28single-precision%29))
  (LocalVariables|SetcurrentPercent (/ (- (Math|Float|Absolute(Float) x) 45.0) 9e+01))
  (if (> (LocalVariables|GetcurrentPercent) 1.0)
    (LocalVariables|SetcurrentPercent 1.0))
  (return (LocalVariables|GetcurrentPercent)))

(fn ChangeWaterLevel
  (params (amount_changed :type Float%20%28single-precision%29) (color :type Linear%20Color%20Structure))
  (bind _capacity (Variables|Default|Getcapacity))
  (bind _returnvalue (/ amount_changed _capacity))
  (bind _output_get (LocalVariables|Setpercent _returnvalue))
  (if (> (+ _returnvalue (/ (Variables|Default|Getamount) (Variables|Default|Getcapacity))) 1.0)
    (LocalVariables|Setpercent (- _output_get (- (+ _returnvalue (/ (Variables|Default|Getamount) (Variables|Default|Getcapacity))) 1.0)))
    (Variables|Default|Setamount (Variables|Default|Getcapacity))
    (else
      (Variables|Default|Setamount (+ amount_changed (Variables|Default|Getamount)))))
  (if (> amount_changed 0.0)
    (CallFunction|ChangeWaterColor color (LocalVariables|Getpercent))))

(fn ChangeWaterColor
  (params (color :type Linear%20Color%20Structure) (percent :type Float%20%28single-precision%29))
  (bind _returnvalue (Rendering|Material|CreateDynamicMaterialInstance (Variables|Default|GetLiquid) 0 (Rendering|Material|GetMaterial (Variables|Default|GetLiquid) 0) "None" :!class /Script/Engine.PrimitiveComponent))
  (bind _output_get (Variables|Default|Setcolor (+ (* color percent) (* (Variables|Default|Getcolor) (- 1.0 percent)))))
  (Rendering|Material|SetVectorParameterValue _returnvalue "Color" _output_get :!class /Script/Engine.MaterialInstanceDynamic)
  (Rendering|Material|SetMaterialbyName (Variables|Default|GetLiquid) "None" _returnvalue))

(fn GetAmount
  (return (Variables|Default|Getamount)))